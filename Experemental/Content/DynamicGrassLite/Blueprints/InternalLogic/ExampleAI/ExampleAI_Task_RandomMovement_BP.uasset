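; Behavior tree task for the example AI that picks a random movement destination near the character stored in the Enemy blackboard key.
; It randomly takes one of that ALS character's formation nav points, though RandomInteger(2) only ever selects the first two of three.
; A random reachable point within a small radius of it is written to DestLocation, and the task finishes successfully.
; A failed cast stops execution without finishing the task.
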(event EventReceiveExecuteAI
  (params (OwnerController :type AI%20Controller%20Object%20Reference) (ControlledPawn :type Pawn%20Object%20Reference))
  (bind _asals_base_character (Utilities|Casting|CastToALS_BaseCharacter (AI|Components|Blackboard|GetValueasObject (AI|GetBlackboard OwnerController) (Utilities|Name|MakeLiteralName "Enemy"))))
  (AI|BehaviorTree|SetBlackboardValueasVector (Variables|Default|GetdestLocation) (.RandomLocation (AI|Navigation|GetRandomReachablePointinRadius (Transformation|GetWorldLocation (Utilities|Array|Get(acopy) (Utilities|Array|MakeArray (Variables|/Game/Geometry/Meshes/AdvancedLocomotionV3/Blueprints/ALS_BaseCharacter.ALS_BaseCharacter_C|GetFormationNavPoint _asals_base_character) (Variables|/Game/Geometry/Meshes/AdvancedLocomotionV3/Blueprints/ALS_BaseCharacter.ALS_BaseCharacter_C|GetFormationNavPoint1 _asals_base_character) (Variables|/Game/Geometry/Meshes/AdvancedLocomotionV3/Blueprints/ALS_BaseCharacter.ALS_BaseCharacter_C|GetFormationNavPoint2 _asals_base_character)) (Math|Random|RandomInteger 2))) 1e+02 0 0)))
  (AI|BehaviorTree|FinishExecute true))