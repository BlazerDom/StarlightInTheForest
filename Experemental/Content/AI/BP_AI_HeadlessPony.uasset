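; Headless pony enemy AI character, driven by a FirstAI controller, with its own resistances, health and randomized gait speeds.
; Tick handles death, blackboard-based target location, periodic sprint toggling and a player line trace that enables its outline when unobstructed.
; A proximity sphere gates repeated attacks, while DamageCollider deals piercing damage scaled by velocity relative to the player.
; AI perception originates from the head sight socket.
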(event OnComponentBeginOverlap(DamageCollider)
  (params (OverlappedComponent :type Primitive%20Component%20Object%20Reference) (OtherActor :type Actor%20Object%20Reference) (OtherComp :type Primitive%20Component%20Object%20Reference) (OtherBodyIndex :type Integer) (bFromSweep :type Boolean) (SweepResult :type Hit%20Result%20Structure%20%28by%20ref%29))
  (Utilities|FlowControl|Delay 0.2)
  (if (Actor|ActorHasTag OtherActor "Player")
    (Utilities|FlowControl|DoOnce false
      (:Completed
        (bind _astest_char (Utilities|Casting|CastToTestChar OtherActor))
        (bind _returnvalue (Physics|GetPhysicsLinearVelocity (Variables|Default|GetDamageCollider) "Neck2_005"))
        (Game|Damage|ApplyDamage _astest_char (/ (Math|Vector|VectorLength (- _returnvalue (Transformation|GetVelocity _astest_char))) 2e+01) 0 0 "/Game/NetworkCharacter/PiercingDamage.PiercingDamage_C")
        (bind _returnvalue_2 (Audio|SpawnSoundAttached "/Game/Effects/Sounds/HitSoundCue.HitSoundCue" (Variables|Character|GetMesh) "DamageCollider" "0, 0, 0" "0, 0, 0" "KeepRelativeOffset" false 1.0 1.0 0.0 0 0))
        (Utilities|IsValid _returnvalue_2
          (:Is%20Valid
            (Effects|Components|ParticleSystem|SetIntParameter _returnvalue_2 "Hits&Vjuh" 0)))))))

(event OnComponentEndOverlap(DamageCollider)
  (params (OverlappedComponent :type Primitive%20Component%20Object%20Reference) (OtherActor :type Actor%20Object%20Reference) (OtherComp :type Primitive%20Component%20Object%20Reference) (OtherBodyIndex :type Integer))
  (if (Actor|ActorHasTag OtherActor "Player")
    (Utilities|FlowControl|DoOnce false) ; enters at Reset
  ))

(event OnComponentBeginOverlap(Sphere1)
  (params (OverlappedComponent :type Primitive%20Component%20Object%20Reference) (OtherActor :type Actor%20Object%20Reference) (OtherComp :type Primitive%20Component%20Object%20Reference) (OtherBodyIndex :type Integer) (bFromSweep :type Boolean) (SweepResult :type Hit%20Result%20Structure%20%28by%20ref%29))
  (if (Actor|ActorHasTag OtherActor "Player")
    (Utilities|FlowControl|Gate true) ; enters at Open
  ))

(event OnComponentEndOverlap(Sphere1)
  (params (OverlappedComponent :type Primitive%20Component%20Object%20Reference) (OtherActor :type Actor%20Object%20Reference) (OtherComp :type Primitive%20Component%20Object%20Reference) (OtherBodyIndex :type Integer))
  (if (Actor|ActorHasTag OtherActor "Player")
    (Utilities|FlowControl|Gate true) ; enters at Close
  ))

(event EventBeginPlay
  (|CallParentFunction)
  (Variables|Default|SetResistForFire 1.0)
  (Variables|Default|SetResistForImpact 0.6)
  (Variables|Default|SetCharacterHP 150)
  (bind _asfirst_ai (Utilities|Casting|CastToFirstAI (Pawn|GetController)))
  (Variables|Default|SetFirst_AI_Ref _asfirst_ai)
  (CallFunction|SetWalkingSpeedEvent (Math|Random|RandomFloatinRange 1.5e+02 2e+02))
  (CallFunction|SetRunningSpeedEvent (Math|Random|RandomFloatinRange 3.5e+02 4e+02))
  (CallFunction|SetSprintingSpeedEvent (Math|Random|RandomFloatinRange 6.2e+02 7e+02))
  (Utilities|FlowControl|Delay 1.0)
  (bind _outactors (Actor|GetAllActorsOfClass "/Game/Geometry/Meshes/AdvancedLocomotionV3/Blueprints/TestChar.TestChar_C"))
  (for _array_element _outactors
    (Variables|Default|SetTestCharRef _array_element)))

(event Collision|EventActorBeginOverlap
  (params (OtherActor :type Actor%20Object%20Reference))
  (|CallParentFunction OtherActor))

(event EventTick
  (params (DeltaSeconds :type Float%20%28single-precision%29))
  (bind _returnvalue (Utilities|Name|MakeLiteralName "Enemy"))
  (bind _returnvalue_2 (AI|GetBlackboard 0))
  (bind _returnvalue_3 (AI|GetBlackboard 0))
  (bind _returnvalue_4 (Utilities|Name|MakeLiteralName "Enemy"))
  (bind _returnvalue_5 (Transformation|GetVelocity))
  (bind _first_ai_ref (Variables|Default|GetFirst_AI_Ref))
  (bind _mesh (Variables|Character|GetMesh))
  (bind _returnvalue_6 (AI|Components|Blackboard|GetValueasObject _returnvalue_2 _returnvalue))
  (bind _returnvalue_7 (AI|Components|Blackboard|GetValueasObject _returnvalue_3 _returnvalue_4))
  (|CallParentFunction DeltaSeconds)
  (if (Variables|Default|GetIsDead)
    (Pawn|Components|CharacterMovement|DisableMovement (Variables|Character|GetCharacterMovement))
    (Variables|/Script/Engine.SkeletalMeshComponent|SetbPauseAnims (Variables|Character|GetMesh) true)
    (Collision|SetCollisionEnabled (Variables|Default|GetBox) "NoCollision")
    (Collision|SetCollisionEnabled (Variables|Default|GetSphere) "NoCollision")
    (Collision|SetCollisionEnabled (Variables|Default|GetSphere1) "NoCollision")
    (Default|Dead _first_ai_ref)
    (AI|Navigation|StopMovement _first_ai_ref)
    (else
      (Utilities|FlowControl|Sequence
        (:then_0
          (Utilities|FlowControl|Gate true
            (:Exit
              (Utilities|FlowControl|DoOnce false :!label _label
                (:Completed
                  (Variables|Default|SetAttackOn? true)
                  (CallFunction|AttackBool false)
                  (Utilities|FlowControl|Delay 0.08)
                  (CallFunction|AttackBool true)
                  (Variables|Default|SetAttackOn? false)
                  (Utilities|FlowControl|Delay 1.0)
                  (goto _label Reset))))))
        (:then_1
          (Utilities|FlowControl|Delay 0.5)
          (CallFunction|LineTrace)
          (if (Variables|Default|GetEnableOutline)
            (Rendering|SetRenderCustomDepth _mesh true)
            (else
              (Rendering|SetRenderCustomDepth _mesh false))))
        (:then_2
          (Utilities|FlowControl|Delay 0.1)
          (CallFunction|CharacterStats))
        (:then_3
          (if (Variables|Default|GetAttackOn?)
            (Utilities|IsValid _returnvalue_6
              (:Is%20Valid
                (bind _asals_base_character (Utilities|Casting|CastToALS_BaseCharacter _returnvalue_6))
                (Variables|Default|SetTargetLocation (+ (Transformation|GetActorLocation _asals_base_character) (Transformation|GetVelocity _asals_base_character) "0,0,20.000000"))))
            (elif (ScalableFloat|GetValueasBool _returnvalue_3 (Utilities|Name|MakeLiteralName "SeeActor"))
              (Utilities|IsValid _returnvalue_7
                (:Is%20Valid
                  (bind _asals_base_character_2 (Utilities|Casting|CastToALS_BaseCharacter _returnvalue_7))
                  (Variables|Default|SetTargetLocation (+ (Transformation|GetActorLocation _asals_base_character_2) _returnvalue_5))))
              (else
                (Variables|Default|SetTargetLocation (+ (AI|Components|Blackboard|GetValueasVector _returnvalue_3 (Utilities|Name|MakeLiteralName "MoveToLocation")) _returnvalue_5))))))
        (:then_4
          (CallFunction|WetCharacter))
        (:then_5
          (CallFunction|MoveRightAxis (Variables|Default|GetMoveAxis))
          (Utilities|FlowControl|Delay (Math|Random|RandomFloatinRange 3.0 5.0))
          (Utilities|FlowControl|FlipFlop
            (:A
              (CallFunction|ActionSprintPressed))
            (:B
              (CallFunction|ActionSprintUnpressed))))
        (:then_6
          (Transformation|SetActorRotation (Variables|Default|GetFirst_AI_Ref) (Variables|Default|GetMouseRotation) true))))))

(fn ConstructionScript
  (|CallParentFunction))

(fn LineTrace
  (bind _testcharref (Variables|Default|GetTestCharRef))
  (Utilities|IsValid _testcharref
    (:Is%20Valid
      (bind (_outhit _returnvalue) (Collision|LineTraceForObjects (Transformation|GetActorLocation) (Transformation|GetActorLocation _testcharref) (Utilities|Array|MakeArray "ObjectTypeQuery1") false (Utilities|Array|MakeArray _testcharref) "None" true "(R=1.000000,G=0.000000,B=0.000000,A=1.000000)" "(R=0.000000,G=1.000000,B=0.000000,A=1.000000)" 1.0))
      (Variables|Default|SetDistanceForTarget (.distance _outhit))
      (if _returnvalue
        (Variables|Default|SetEnableOutline false)
        (else
          (Variables|Default|SetEnableOutline true))))))

(fn GetPerceptionLocRot
  (bind _mesh (Variables|Character|GetMesh))
  (bind _returnvalue (Transformation|GetSocketTransform _mesh "HeadSightSocket" "RTS_World"))
  (bind (_location _rotation) (Math|Transform|BreakTransform _returnvalue))
  (return _location _rotation))