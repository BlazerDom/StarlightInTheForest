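; AI-controlled mage character that casts rune-combination spells (fireball, front fireball, flame, freeze stop) and respawns at a random PlayerStart after death.
; On overlap, the server spawns and attaches a BP_MagePawn once, sharing it with the FirstAI controller.
; Cast events send timed rune calls to that pawn.
; Delay-throttled Tick updates stats and outlines the mesh when a WorldStatic trace to the blackboard Enemy is unobstructed.
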(event Custom|CastFireBallInFront
  (bind _bp_magepawnairef (Variables|Default|GetBP_MagePawnAIRef))
  (Networking|SwitchHasAuthority
    (:Authority
      (Utilities|FlowControl|Delay 0.1)
      (Default|Server:FireRune(Kano) _bp_magepawnairef)
      (Utilities|FlowControl|Delay 0.2)
      (Default|Server:TransformRune(Ingwaz) _bp_magepawnairef)
      (Utilities|FlowControl|Delay 0.2)
      (Default|Server:launchRune(Raido) _bp_magepawnairef))))

(event Custom|CastFireBoll
  (bind _bp_magepawnairef (Variables|Default|GetBP_MagePawnAIRef))
  (Networking|SwitchHasAuthority
    (:Authority
      (Default|Server:FireRune(Kano) _bp_magepawnairef)
      (Utilities|FlowControl|Delay 0.2)
      (Default|Server:ListeningRune(Ancuz) _bp_magepawnairef))))

(event Custom|CastFireFlame
  (bind _bp_magepawnairef (Variables|Default|GetBP_MagePawnAIRef))
  (Networking|SwitchHasAuthority
    (:Authority
      (Default|Server:FireRune(Kano) _bp_magepawnairef)
      (Utilities|FlowControl|Delay 0.2)
      (Default|Server:FireRune(Kano) _bp_magepawnairef)
      (Utilities|FlowControl|Delay 0.2)
      (Default|Server:launchRune(Raido) _bp_magepawnairef))))

(event Custom|CastStop
  (Networking|SwitchHasAuthority
    (:Authority
      (Default|Server:FreezeRune(Isa) (Variables|Default|GetBP_MagePawnAIRef)))))

(event Collision|EventActorBeginOverlap
  (params (OtherActor :type Actor%20Object%20Reference))
  (Variables|Default|SetThisAI? true)
  (|CallParentFunction OtherActor)
  (Utilities|FlowControl|DoOnce false
    (:Completed
      (Networking|SwitchHasAuthority
        (:Authority
          (bind _returnvalue (Game|SpawnActorfromClass "/Game/NetworkCharacter/BP_MagePawn.BP_MagePawn_C" (Transformation|GetActorTransform) "Undefined" 0 0 0))
          (Transformation|AttachActorToActor _returnvalue self "None" "KeepWorld" "KeepWorld" "KeepWorld" true)
          (Variables|Default|SetBP_MagePawnAIRef _returnvalue)
          (bind _asfirst_ai (Utilities|Casting|CastToFirstAI (AI|GetAIController 0)))
          (Variables|/Game/AI/FirstAI.FirstAI_C|SetBP_MagePawnAIRef _asfirst_ai (Variables|Default|GetBP_MagePawnAIRef))
          (Variables|/Game/NetworkCharacter/BP_MagePawn.BP_MagePawn_C|SetServerCharacterRef (Variables|Default|GetBP_MagePawnAIRef) self)
          (Variables|/Game/NetworkCharacter/BP_MagePawn.BP_MagePawn_C|SetThisIsAI (Variables|Default|GetBP_MagePawnAIRef) true))))))

(event EventTick
  (params (DeltaSeconds :type Float%20%28single-precision%29))
  (bind _mesh (Variables|Character|GetMesh))
  (|CallParentFunction 0.0)
  (Utilities|FlowControl|Sequence
    (:then_0
      (Utilities|FlowControl|Delay 0.1)
      (CallFunction|CharacterStats)
      (if (Variables|Default|GetEnableOutline)
        (Rendering|SetRenderCustomDepth _mesh true)
        (else
          (Rendering|SetRenderCustomDepth _mesh false))))
    (:then_1
      (if (Variables|Default|GetIsDead_0)
        (Utilities|FlowControl|Delay 3.0)
        (bind _outactors (Actor|GetAllActorsOfClass "/Script/Engine.PlayerStart"))
        (Transformation|SetActorLocation (Transformation|GetActorLocation (Utilities|Array|Get(acopy) _outactors (Math|Random|RandomIntegerinRange 0 (Utilities|Array|LastIndex _outactors)))) false true)
        (Variables|Default|SetCharacterHP_0 100)
        (Variables|Default|SetIsDead_0 false)))
    (:then_2
      (Utilities|FlowControl|Delay 0.2)
      (CallFunction|LineTrace))))

(fn ConstructionScript
  (|CallParentFunction))

(fn LineTrace
  (bind _returnvalue (AI|GetBlackboard 0))
  (bind _returnvalue_2 (Utilities|Name|MakeLiteralName "Enemy"))
  (bind _returnvalue_3 (AI|Components|Blackboard|GetValueasObject _returnvalue _returnvalue_2))
  (if (== _returnvalue_3 0)
    (Variables|Default|SetEnableOutline false)
    (else
      (bind _astest_char (Utilities|Casting|CastToTestChar _returnvalue_3))
      (bind _returnvalue_4 (Collision|LineTraceForObjects (Transformation|GetActorLocation) (Transformation|GetActorLocation _astest_char) (Utilities|Array|MakeArray "ObjectTypeQuery1") false 0 "None" true "(R=1.000000,G=0.000000,B=0.000000,A=1.000000)" "(R=0.000000,G=1.000000,B=0.000000,A=1.000000)" 1.0))
      (if _returnvalue_4
        (Variables|Default|SetEnableOutline false)
        (else
          (Variables|Default|SetEnableOutline true))))))