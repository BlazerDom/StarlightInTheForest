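; BP_MagePawn_AI is a mage AI Blueprint that creates a server-side character counterpart for itself.
; On BeginPlay, only the authority spawns a ServerCharacterController actor at this actor's transform and stores it in ServerSideCharacterRef.
; A disconnected fragment for handing that reference to an AI and possessing it never runs, and the construction script only calls its parent.
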(event EventBeginPlay
  (Networking|SwitchHasAuthority
    (:Authority
      (bind _returnvalue (Game|SpawnActorfromClass "/Game/Blueprint/OldTest/ServerCharacterController.ServerCharacterController_C" (Transformation|GetActorTransform) "Undefined" 0 0))
      (Variables|Default|SetServerSideCharacterRef _returnvalue))))

(fn ConstructionScript
  (|CallParentFunction))