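; Mage pawn that casts rune-based fire and water magic on the server.
; Rune events append letters to SpellTable, which clears after a retriggerable delay, then run fire and water activity.
; Tick captures overlapping magic on matching spell words and steers water toward the mouse location.
; Water spells match words for icicles, fog, shields and freezing; fire actors receive the raw string; traces set and range-check a missile target.
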(event Custom|Server:FireActivity
  ;[1 0 0] Execution spells
  (Networking|SwitchHasAuthority
    (:Authority
      (for _array_element (Variables|Default|GetMyFires)
        (Utilities|IsValid _array_element
          (:Is%20Valid
            (bind _asfire (Utilities|Casting|CastToFire _array_element))
            (Default|FireListen _asfire (Variables|Spell|GetSpellTable))))))))

(event Custom|Server:launchRune%28Raido%29
  (Rune|LaunchRuneActive(Raido)'R'or'D')
  (CallFunction|Server:FireActivity)
  (CallFunction|Server:WaterActivity)
  (Utilities|FlowControl|RetriggerableDelay 3.0)
  (Variables|Spell|SetSpellTable ""))

(event Custom|Server:WaterRune%28Lagus%29
  (Rune|WaterRuneActive(Largus)'L')
  (CallFunction|Server:FireActivity)
  (CallFunction|Server:WaterActivity)
  (Utilities|FlowControl|RetriggerableDelay 3.0)
  (Variables|Spell|SetSpellTable ""))

(event Custom|Server:WaterActivity
  (bind _mywater (Variables|Default|GetMyWater))
  (if (> (Utilities|String|Len (Variables|Spell|GetSpellTable)) 2)
    (Networking|SwitchHasAuthority
      (:Authority
        (Utilities|FlowControl|Sequence
          (:then_0
            (for (_array_element _array_index) _mywater
              (Utilities|IsValid _array_element
                (:Is%20Valid
                  (Variables|Default|SetOverlappingArrayInt _array_index)
                  (if (> (Variables|Default|GetOverlappingArrayInt) -1)
                    (Variables|Default|SetOverlappingArrayInt (- (Variables|Default|GetOverlappingArrayInt) 1))
                    (bind _aswater_ball (Utilities|Casting|CastToWaterBall _array_element))
                    (if (Variables|/Game/Blueprint/WorldMagic/Water/WaterBall.WaterBall_C|GetTransformActive? _aswater_ball)
                      (Utilities|FlowControl|Sequence
                        (:then_0
                          (CallFunction|UnfreezeIcicle _array_element "LIG" :!label _label)
                          (if (Variables|/Game/Blueprint/WorldMagic/Water/WaterBall.WaterBall_C|GetBubbleShieldActive? _aswater_ball)
                            (CallFunction|BubbleShield _array_element "WZG" false)))
                        (:then_1
                          (if (not (or (Variables|/Game/Blueprint/WorldMagic/Water/WaterBall.WaterBall_C|GetShieldActive? _aswater_ball) (Variables|/Game/Blueprint/WorldMagic/Water/WaterBall.WaterBall_C|GetSword? _aswater_ball)))
                            (bind _aswater (Utilities|SpellWordforWater _array_element "LIR" :!label _label_2))
                            (Default|LaunchMiniIcicle _aswater)
                            (Variables|Spell|SetSpellTable "")))
                        (:then_2
                          (CallFunction|IcicleLaunch _array_element "LTR" :!label _label_3)))
                      (else
                        (Utilities|FlowControl|Sequence
                          (:then_0
                            (Utilities|WaterIcicleMacros _array_element "LWI"))
                          (:then_1
                            (goto _label_3))
                          (:then_2
                            (goto _label))
                          (:then_3
                            (CallFunction|MakeFog _array_element "LWZR" true))
                          (:then_4
                            (CallFunction|MakeFog _array_element "LWG" false))
                          (:then_5
                            (if (not (Variables|Default|GetBubbleAcive?))
                              (CallFunction|MakeShieldorSword _array_element "WIIBI" false)))
                          (:then_6
                            (goto _label_2))
                          (:then_7
                            (CallFunction|BubbleShield _array_element "LWMZ" true)))))))
                (:Is%20Not%20Valid
                  (Utilities|Array|RemoveIndex _mywater _array_index)))))
          (:then_1
            (CallFunction|FreezeAll "LWMI")))))))

(event Custom|Server:DisableRune%28Gebo%29
  (Rune|DisableRuneActive(Gebo)'G')
  (CallFunction|Server:FireActivity)
  (CallFunction|Server:WaterActivity)
  (Utilities|FlowControl|RetriggerableDelay 3.0)
  (Variables|Spell|SetSpellTable ""))

(event Custom|Server:TargertRune%28Mannaz%29
  (params (NazOr%20Man :type Boolean))
  (Rune|TragetRuneActive(Mannaz)'M'Or'N' NazOr%20Man)
  (CallFunction|Server:FireActivity)
  (CallFunction|Server:WaterActivity)
  (Utilities|FlowControl|RetriggerableDelay 3.0)
  (Variables|Spell|SetSpellTable ""))

(event Custom|Server:ProtectionRune%28Algiz%29
  (Rune|ProtectionRuneActive(Algiz)'Z')
  (CallFunction|Server:FireActivity)
  (CallFunction|Server:WaterActivity)
  (Utilities|FlowControl|RetriggerableDelay 3.0)
  (Variables|Spell|SetSpellTable ""))

(event Custom|Server:DirectionRune%28Teivaz%29
  (params (VazOrTai :type Boolean))
  (Rune|DirectionRuneActive(Teivaz)'T'Or'V VazOrTai)
  (CallFunction|Server:FireActivity)
  (CallFunction|Server:WaterActivity)
  (Utilities|FlowControl|RetriggerableDelay 3.0)
  (Variables|Spell|SetSpellTable ""))

(event Custom|Server:FireRune%28Kano%29
  (Rune|FireRuneActive(Kano)'K')
  (CallFunction|Server:FireActivity)
  (CallFunction|Server:WaterActivity)
  (Utilities|FlowControl|RetriggerableDelay 3.0)
  (Variables|Spell|SetSpellTable ""))

(event Custom|Server:TransformRune%28Ingwaz%29
  (Rune|TransformRuneActive(Ingwaz)'W')
  (CallFunction|Server:FireActivity)
  (CallFunction|Server:WaterActivity)
  (Utilities|FlowControl|RetriggerableDelay 3.0)
  (Variables|Spell|SetSpellTable ""))

(event Custom|Server:FireControll
  (bind _migicoverlap (Utilities|MagicSpawn&Controll 0 "K" "/Game/Blueprint/WorldMagic/Fire/Fire.Fire_C")
    (:CaptureMagicAI
      (if (== (Utilities|GetClass _migicoverlap) "/Game/Blueprint/WorldMagic/Fire/FireBall.FireBall_C")
        (Fire|CaptureFireforAI _migicoverlap)))
    (:CaptureMagicPlayer
      (bind _asfire (Utilities|Casting|CastToFire _migicoverlap :!label _label))
      (Default|FireListening _asfire self)
      (Utilities|Array|AddUnique (Variables|Default|GetMyFires) _migicoverlap))
    (:true
      (goto _label))))

(event Custom|Server:ListeningRune%28Ancuz%29
  (Rune|ListeningRuneActive(Ancuz)'A')
  (CallFunction|Server:FireActivity)
  (CallFunction|Server:WaterActivity)
  (Utilities|FlowControl|RetriggerableDelay 3.0)
  (Variables|Spell|SetSpellTable ""))

(event Custom|Server:FreezeRune%28Isa%29
  (Rune|FreezeRuneActive(Isa)'I')
  (CallFunction|Server:FireActivity)
  (CallFunction|Server:WaterActivity)
  (Utilities|FlowControl|RetriggerableDelay 3.0)
  (Variables|Spell|SetSpellTable ""))

(event Custom|TakeTarget
  (Utilities|FlowControl|Delay 0.2)
  (Networking|SwitchHasAuthority
    (:Authority
      (bind _outhit (Collision|SphereTraceForObjects (Transformation|GetActorLocation) (+ (Variables|/Game/Blueprint/CharacterControllers/ClientSideController.ClientSideController_C|GetMouseLocation (Variables|Default|GetClientSideControllerRef)) "0,0.000000,30.000000") 2e+02 (Utilities|Array|MakeArray "ObjectTypeQuery3" "ObjectTypeQuery1") false (Utilities|Array|MakeArray (Variables|/Game/Blueprint/CharacterControllers/ClientSideController.ClientSideController_C|GetServerSideCharacterRef (Variables|Default|GetClientSideControllerRef))) "None" true "(R=1.000000,G=0.000000,B=0.000000,A=1.000000)" "(R=0.000000,G=1.000000,B=0.000000,A=1.000000)" 0.2))
      (if true
        (if (or (== (Utilities|GetClass (.HitActor (Collision|BreakHitResult _outhit))) "/Game/Blueprint/OldTest/ServerCharacterController.ServerCharacterController_C") (== (Utilities|GetClass (.HitActor (Collision|BreakHitResult _outhit))) "/Game/AI/BP_AICharecter.BP_AICharecter_C"))
          (bind _output_get (Variables|Default|SetTargetForMissile (.HitActor (Collision|BreakHitResult _outhit))))
          (Development|PrintString (Utilities|GetDisplayName _output_get)))))))

(event Custom|RangeToTarget
  (bind _returnvalue (Transformation|GetActorLocation))
  (Utilities|FlowControl|Delay 0.5)
  (if (not (== (Variables|Default|GetTargetForMissile) 0))
    (bind _returnvalue_2 (Collision|LineTraceForObjects _returnvalue (Transformation|GetActorLocation (Variables|Default|GetTargetForMissile)) (Utilities|Array|MakeArray "ObjectTypeQuery1") false 0 "None" true "(R=1.000000,G=0.000000,B=0.000000,A=1.000000)" "(R=0.000000,G=1.000000,B=0.000000,A=1.000000)" 0.2))
    (if (or (> (Math|Vector|VectorLength (- _returnvalue (Transformation|GetActorLocation (Variables|Default|GetTargetForMissile)))) 1e+03) _returnvalue_2)
      (Utilities|FlowControl|Delay 1.0)
      (Variables|Default|SetTargetForMissile 0)
      (Development|PrintString "target out of range"))))

(event Custom|Server:WaterControll
  (bind _mywater (Variables|Default|GetMyWater))
  (bind _migicoverlap (Utilities|MagicSpawn&Controll "/Game/Blueprint/WorldMagic/Water/WaterBall.WaterBall_C" "LMR" "/Game/Blueprint/WorldMagic/Water/WaterBall.WaterBall_C")
    (:CaptureMagicPlayer
      (if (== (Utilities|GetClass _migicoverlap) "/Game/Blueprint/WorldMagic/Water/WaterBall.WaterBall_C")
        (CallFunction|WaterCapture _migicoverlap)))
    (:RotationControllForPlayer
      (if (== (Utilities|GetClass _migicoverlap) "/Game/Blueprint/WorldMagic/Water/WaterBall.WaterBall_C")
        (if (> (Utilities|Array|LastIndex _mywater) -1)
          (for (_array_element _array_index) _mywater
            (Utilities|IsValid _array_element
              (:Is%20Valid
                (CallFunction|WaterRotation _array_element))
              (:Is%20Not%20Valid
                (Utilities|Array|RemoveIndex _mywater _array_index)))))))))

(event EventTick
  (params (DeltaSeconds :type Float%20%28single-precision%29))
  (Utilities|FlowControl|Sequence
    (:then_0
      (CallFunction|RangetoTarget))
    (:then_1
      (Utilities|FlowControl|Sequence
        (:then_0
          (CallFunction|Server:FireControll))
        (:then_1
          (CallFunction|Server:WaterControll))))
    (:then_2
      (if (Variables|Default|GetThisIsAI)
        _))))

(fn ConstructionScript)

(fn FireRuneActive(Kano)'K'
  (bind _output_get (Variables|Spell|SetSpellTable (Utilities|String|Append (Variables|Spell|GetSpellTable) "K"))))

(fn TransformRuneActive(Ingwaz)'W'
  (bind _output_get (Variables|Spell|SetSpellTable (Utilities|String|Append (Variables|Spell|GetSpellTable) "W")))
  (Audio|PlaySoundatLocation 0 (Transformation|GetActorLocation) "0, 0, 0" 1.0 1.0 0.0 0 0 0))

(fn LaunchRuneActive(Raido)'R'or'D'
  (if false
    (bind _output_get (Variables|Spell|SetSpellTable (Utilities|String|Append (Variables|Spell|GetSpellTable) "D")))
    (else
      (bind _output_get_2 (Variables|Spell|SetSpellTable (Utilities|String|Append (Variables|Spell|GetSpellTable) "R"))))))

(fn ListeningRuneActive(Ancuz)'A'
  (bind _output_get (Variables|Spell|SetSpellTable (Utilities|String|Append (Variables|Spell|GetSpellTable) "A"))))

(fn CaptureFire
  (params (OverlappingActor :type Actor%20Object%20Reference))
  (bind _output_get (Variables|Default|SetOverlappingActor OverlappingActor))
  (if (Utilities|Enum|Equal(Enum) (Variables|Spell|GetSpellTable) "FA")
    (Utilities|Casting|CastToFireBall _output_get)))

(fn FireBallCompil
  (params (OverlappingActor :type Actor%20Object%20Reference))
  (bind _output_get (Variables|Default|SetOverlappingActor OverlappingActor))
  (bind _asfire_ball (Utilities|Casting|CastToFireBall _output_get))
  (for (_array_element _array_index) (Collision|GetOverlappingActors _asfire_ball "/Game/Blueprint/WorldMagic/Fire/FireBall.FireBall_C" :!class /Script/Engine.Actor)
    (if (not (>= (* (Variables|/Game/Blueprint/WorldMagic/Fire/FireBall.FireBall_C|GetFireBatarySettings _asfire_ball) 0.26) 33.0))
      (Actor|DestroyActor _array_element)
      (if (>= _array_index 0)
        (Default|FireBallCompil _asfire_ball)))))

(fn FreezeRuneActive(Isa)'I'
  (bind _output_get (Variables|Spell|SetSpellTable (Utilities|String|Append (Variables|Spell|GetSpellTable) "I"))))

(fn FireBallRotation
  (params (TargetForRot :type Fire%20Ball%20Object%20Reference) (SpawnActorLocation :type Actor%20Object%20Reference) (CoordinateSet? :type Boolean) (AlwaseSetCoord :type Boolean))
  (bind _clientsidecontrollerref (Variables|Default|GetClientSideControllerRef))
  (bind _mouselocation (Variables|/Game/Blueprint/CharacterControllers/ClientSideController.ClientSideController_C|GetMouseLocation _clientsidecontrollerref))
  (if CoordinateSet?
    (Default|FireRotation TargetForRot (stale _output_get_2) 0.0 :!label _label)
    (else
      (bind _output_get (Variables|Default|SetNewVar_0 (Math|Vector|VectorLength (- (Transformation|GetActorLocation SpawnActorLocation) _mouselocation))))
      (bind _output_get_2 (Variables|Default|SetRotationCoordinate (+ _mouselocation (Math|Vector|MakeVector 0.0 0.0 (/ _output_get 4.0)))))
      (if AlwaseSetCoord
        (goto _label)))))

(fn OnRepTargetforMissile)

(fn CaptureFireforAI
  (params (OverlappingActor :type Actor%20Object%20Reference))
  (bind _output_get (Variables|Default|SetOverlappingActor OverlappingActor))
  (Utilities|Casting|CastToFireBall _output_get))

(fn FireBallRotationforAI
  (params (OverlappingActor :type Actor%20Object%20Reference))
  (bind _returnvalue (Utilities|Name|MakeLiteralName "Enemy"))
  (bind _firstairef (Variables|Default|GetFirstAIRef))
  (bind _returnvalue_2 (AI|GetBlackboard _firstairef))
  (bind _resultlocation (Class|BlackboardComponent|GetLocationfromEntry _returnvalue_2 _returnvalue))
  (Utilities|FlowControl|Sequence
    (:then_0
      (if (Variables|Default|GetFlameON)
        (Variables|Default|SetAITargetVelocity "0, 0, 0")
        (else
          (bind _asserver_character_controller (Utilities|Casting|CastToServerCharacterController (AI|Components|Blackboard|GetValueasObject (AI|GetBlackboard (Variables|Default|GetFirstAIRef)) (Utilities|Name|MakeLiteralName "Enemy"))))
          (Variables|Default|SetAITargetVelocity (Transformation|GetVelocity _asserver_character_controller)))))
    (:then_1
      (bind _output_get (Variables|Default|SetOverlappingActor OverlappingActor))
      (bind _asfire_ball (Utilities|Casting|CastToFireBall _output_get))
      (bind _output_get_2 (Variables|Default|SetNewVar_0 (Math|Vector|VectorLength (- (Transformation|GetActorLocation) _resultlocation))))
      (Default|FireRotation _asfire_ball (+ (Variables|Default|GetAITargetVelocity) (+ _resultlocation (Math|Vector|MakeVector 0.0 0.0 (/ _output_get_2 1e+01)))) 0.0))))

(fn WaterCapture
  (params (OverlappingActor :type Actor%20Object%20Reference))
  (bind _output_get (Variables|Default|SetOverlappingActor OverlappingActor))
  (bind _aswater_ball (Utilities|Casting|CastToWaterBall _output_get))
  (Utilities|Array|AddUnique (Variables|Default|GetMyWater) _aswater_ball)
  (Default|HomingMissile _aswater_ball (Variables|/Game/Blueprint/CharacterControllers/ClientSideController.ClientSideController_C|GetServerSideCharacterRef (Variables|Default|GetClientSideControllerRef)) self true))

(fn WaterCaptureforAI)

(fn WaterRotation
  (params (OverlappingActor :type Actor%20Object%20Reference))
  (bind _clientsidecontrollerref (Variables|Default|GetClientSideControllerRef))
  (bind _mouselocation (Variables|/Game/Blueprint/CharacterControllers/ClientSideController.ClientSideController_C|GetMouseLocation _clientsidecontrollerref))
  (bind _output_get (Variables|Default|SetOverlappingActor OverlappingActor))
  (bind _aswater_ball (Utilities|Casting|CastToWaterBall _output_get))
  (if (Variables|/Game/Blueprint/WorldMagic/Water/WaterBall.WaterBall_C|GetIcicleON _aswater_ball)
    (Default|WaterRotation _aswater_ball (+ _mouselocation "0, 0,50.000000"))
    (else
      (Default|WaterRotation _aswater_ball _mouselocation))))

(fn WaterRuneActive(Largus)'L'
  (bind _output_get (Variables|Spell|SetSpellTable (Utilities|String|Append (Variables|Spell|GetSpellTable) "L"))))

(fn IcicleLaunch
  (params (OverlappingActor :type Actor%20Object%20Reference) (IcicleLaunchWord :type String))
  (Utilities|FlowControl|DoOnce false
    (:Completed
      (bind _output_get (Variables|Default|SetOverlappingActor OverlappingActor))
      (if (Utilities|String|EndsWith (Variables|Spell|GetSpellTable) IcicleLaunchWord)
        (bind _aswater_ball (Utilities|Casting|CastToWaterBall _output_get))
        (if (Variables|/Game/Blueprint/WorldMagic/Water/WaterBall.WaterBall_C|GetIcicleON _aswater_ball)
          (Default|HomingMissileOff _aswater_ball))))))

(fn UnfreezeIcicle
  (params (OverlappingActor :type Actor%20Object%20Reference) (UnfreezeWord :type String))
  (bind _output_get (Variables|Default|SetOverlappingActor OverlappingActor))
  (if (Utilities|String|EndsWith (Variables|Spell|GetSpellTable) UnfreezeWord)
    (bind _aswater_ball (Utilities|Casting|CastToWaterBall _output_get))
    (Default|Unfreeze _aswater_ball (Variables|/Game/Blueprint/CharacterControllers/ClientSideController.ClientSideController_C|GetServerSideCharacterRef (Variables|Default|GetClientSideControllerRef)))))

(fn FreezeAll
  (params (SpellWord :type String))
  (if (Utilities|String|Contains (Variables|Spell|GetSpellTable) SpellWord false true)
    (for _array_element (Variables|Default|GetActorsOverlap)
      (bind _asals_base_character (Utilities|Casting|CastToALS_BaseCharacter _array_element))
      (if (Variables|/Game/Geometry/Meshes/AdvancedLocomotionV3/Blueprints/ALS_BaseCharacter.ALS_BaseCharacter_C|GetIsWet _asals_base_character)
        (Default|FreezeCharacter _asals_base_character)))))

(fn MakeFog
  (params (OverlappingActor :type Actor%20Object%20Reference) (SpellWord :type String) (FogOn? :type Boolean))
  (bind _output_get (Variables|Default|SetOverlappingActor OverlappingActor))
  (if (Utilities|String|EndsWith (Variables|Spell|GetSpellTable) SpellWord)
    (bind _aswater_ball (Utilities|Casting|CastToWaterBall _output_get))
    (if (Math|Boolean|NotEqual(Boolean) FogOn? (Components|Activation|IsActive (Variables|/Game/Blueprint/WorldMagic/Water/WaterBall.WaterBall_C|GetFog _aswater_ball)))
      (Default|FogActivate? _aswater_ball FogOn?)
      (Variables|Spell|SetSpellTable ""))))

(fn MakeShieldorSword
  (params (OverlappingActor :type Actor%20Object%20Reference) (SpellWord :type String) (IfTrueShildOff&SwordOn :type Boolean))
  (bind _self self)
  (bind _clientsidecontrollerref (Variables|Default|GetClientSideControllerRef))
  (bind _serversidecharacterref (Variables|/Game/Blueprint/CharacterControllers/ClientSideController.ClientSideController_C|GetServerSideCharacterRef _clientsidecontrollerref))
  (bind _output_get (Variables|Default|SetOverlappingActor OverlappingActor))
  (if (Utilities|Enum|Equal(Enum) (Variables|Spell|GetSpellTable) SpellWord)
    (bind _aswater_ball (Utilities|Casting|CastToWaterBall _output_get))
    (if IfTrueShildOff&SwordOn
      (Default|IceSword _aswater_ball _serversidecharacterref _self)
      (else
        (Default|IceShield _aswater_ball _serversidecharacterref _self)))))

(fn BubbleShield
  (params (OverlappingActor :type Actor%20Object%20Reference) (SpellWord :type String) (BubbleShieldOn? :type Boolean))
  (bind _output_get (Variables|Default|SetOverlappingActor OverlappingActor))
  (if (Utilities|String|EndsWith (Variables|Spell|GetSpellTable) SpellWord)
    (bind _aswater_ball (Utilities|Casting|CastToWaterBall _output_get))
    (Variables|Default|SetBubbleAcive? BubbleShieldOn?)
    (Default|BubbleShield _aswater_ball BubbleShieldOn? (Variables|/Game/Blueprint/CharacterControllers/ClientSideController.ClientSideController_C|GetServerSideCharacterRef (Variables|Default|GetClientSideControllerRef)) self)))

(fn DirectionRuneActive(Teivaz)'T'Or'V
  (params (VazOrTai :type Boolean))
  (if VazOrTai
    (bind _output_get (Variables|Spell|SetSpellTable (Utilities|String|Append (Variables|Spell|GetSpellTable) "V")))
    (else
      (bind _output_get_2 (Variables|Spell|SetSpellTable (Utilities|String|Append (Variables|Spell|GetSpellTable) "T")))))
  (Audio|PlaySoundatLocation 0 (Transformation|GetActorLocation) "0, 0, 0" 1.0 1.0 0.0 0 0 0))

(fn DisableRuneActive(Gebo)'G'
  (bind _output_get (Variables|Spell|SetSpellTable (Utilities|String|Append (Variables|Spell|GetSpellTable) "G")))
  (Audio|PlaySoundatLocation 0 (Transformation|GetActorLocation) "0, 0, 0" 1.0 1.0 0.0 0 0 0))

(fn ProtectionRuneActive(Algiz)'Z'
  (bind _output_get (Variables|Spell|SetSpellTable (Utilities|String|Append (Variables|Spell|GetSpellTable) "Z")))
  (Audio|PlaySoundatLocation 0 (Transformation|GetActorLocation) "0, 0, 0" 1.0 1.0 0.0 0 0 0))

(fn TragetRuneActive(Mannaz)'M'Or'N'
  (params (NazOr%20Man :type Boolean))
  (if NazOr%20Man
    (bind _output_get (Variables|Spell|SetSpellTable (Utilities|String|Append (Variables|Spell|GetSpellTable) "N")))
    (else
      (bind _output_get_2 (Variables|Spell|SetSpellTable (Utilities|String|Append (Variables|Spell|GetSpellTable) "M"))))))