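; Lightning storm world element that creates recurring thunder and lightning flashes at random intervals.
; Tick feeds a random-length Delay, which acts as a repeating timer for the lightning event.
; Each strike plays thunder at a random XY location, briefly waits, then turns the directional light to a random yaw.
; A timeline then drives the light's intensity to produce the flash.
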(event Custom|LightningEvent
  (bind _returnvalue (Math|Random|RandomFloatinRange 0.0 1.1e+04))
  (Audio|PlaySoundatLocation "/Game/Effects/Sounds/ThunderBlast/ThunderCue.ThunderCue" (Math|Vector|MakeVector _returnvalue _returnvalue 1e+02) "0, 0, 0" 1.0 1.0 0.5 0 0 0)
  (Utilities|FlowControl|Delay 0.2)
  (Transformation|SetWorldRotation (Variables|Default|GetDirectionalLight) (Math|Rotator|MakeRotator -1.2e+02 -4e+01 (Math|Random|RandomFloatinRange -3.6e+02 3.6e+02)) false false)
  (bind _luxintensive (Timeline|Lightning PlayFromStart)
    (:Update
      (Rendering|Components|Light|SetIntensity (Variables|Default|GetDirectionalLight) _luxintensive))))

(event Collision|EventActorBeginOverlap
  (params (OtherActor :type Actor%20Object%20Reference)))

(event EventTick
  (params (DeltaSeconds :type Float%20%28single-precision%29))
  (Utilities|FlowControl|Delay (Math|Random|RandomFloatinRange 0.3 1e+01))
  (CallFunction|LightningEvent))

(fn ConstructionScript)