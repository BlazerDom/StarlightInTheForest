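; Test character Blueprint that tracks health and death state and exposes movement and animation-flag helpers.
; AnyDamage subtracts only FireDamage from CharacterHP, truncates to an integer and prints it.
; A separate CharacterStats event, not called here, updates IsDead from HP after a short delay.
; Functions set walk speed and acceleration, apply a fixed minimum speed, or set the SetStop and IsDead flags.
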(event Custom|CharacterStats
  (Utilities|FlowControl|Delay 0.1)
  (Variables|Default|SetIsDead (<= (Variables|Stats|GetCharacterHP) 0)))

(event EventTick
  (params (DeltaSeconds :type Float%20%28single-precision%29)))

(event Game|Damage|EventAnyDamage
  (params (Damage :type Float%20%28single-precision%29) (DamageType :type Damage%20Type%20Object%20Reference) (InstigatedBy :type Controller%20Object%20Reference) (DamageCauser :type Actor%20Object%20Reference))
  (Utilities|Casting|CastToFireDamage DamageType)
  (bind _output_get (Variables|Stats|SetCharacterHP (Math|Float|Truncate (- (Math|Conversions|ToFloat(Integer) (Variables|Stats|GetCharacterHP)) Damage))))
  (Development|PrintString (Utilities|String|BuildString(Integer) "Health  " "" _output_get)))

(fn ConstructionScript)

(fn MaxWalkSpeed
  (params (MaxWalkSpeed :type Float%20%28single-precision%29) (MaxAcceleration :type Float%20%28single-precision%29))
  (bind _charactermovement (Variables|Character|GetCharacterMovement))
  (Variables|/Script/Engine.CharacterMovementComponent|SetMaxWalkSpeed _charactermovement MaxWalkSpeed)
  (Variables|/Script/Engine.CharacterMovementComponent|SetMaxAcceleration _charactermovement MaxAcceleration))

(fn MinWalkSpeed
  (Variables|/Script/Engine.CharacterMovementComponent|SetMaxWalkSpeed (Variables|Character|GetCharacterMovement) 1.5e+02))

(fn StopMoveAnim
  (params (SetStop :type Boolean))
  (Variables|Default|SetSetStop SetStop))

(fn Dead
  (params (IsDead? :type Boolean))
  (Variables|Default|SetIsDead IsDead?))