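; BP_MagePawn is a networked mage pawn that casts fire and water spells by combining runes.
; Rune events append letters to SpellTable, which server-authority activity handlers match against spell words, clearing it after a one-second retriggerable delay.
; Tick-driven control events capture overlapping Fire and Water actors and steer water toward the mouse.
; Spells launch missiles at a traced, range-checked target, toggle flame and fog, form icicles or shields, and freeze wet characters.
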(event Custom|Server:FireActivity
  (Networking|SwitchHasAuthority
    (:Authority
      (for _array_element (Collision|GetOverlappingActors "/Game/WorldMagicElements/Fire.Fire_C" :!class /Script/Engine.Actor)
        (Utilities|FlowControl|Sequence
          (:then_0
            (if (Utilities|Enum|Equal(Enum) (Variables|Spell|GetSpellTable) "FHBA")
              (bind _asfire_ball (Utilities|Casting|CastToFireBall _array_element))
              (Default|SpawnMissile _asfire_ball (Variables|Default|GetTargetForMissile))
              (Variables|Spell|SetSpellTable "")))
          (:then_1
            (Utilities|FlowControl|Delay 0.05)
            (Utilities|CorrectSpellWord "FBH"
              (:true
                (Variables|Spell|SetFireBallLaunch true)
                (Utilities|FlowControl|Delay 0.06)
                (Variables|Spell|SetSpellTable "")
                (Variables|Spell|SetFireBallLaunch false))))
          (:then_2
            (Utilities|CorrectSpellWord "FFH"
              (:true
                (Variables|Default|SetFlameON true)
                (Variables|Spell|SetSpellTable "" :!label _label))))
          (:then_3
            (Utilities|CorrectSpellWord "IF"
              (:true
                (Variables|Default|SetFlameON false)
                (goto _label)))))))))

(event Custom|Server:ForwardRune%28Hagalaz%29
  (Rune|ForwardRuneActive(Hagalaz))
  (CallFunction|Server:FireActivity)
  (CallFunction|Server:WaterActivity)
  (Utilities|FlowControl|RetriggerableDelay 1.0)
  (Variables|Spell|SetSpellTable ""))

(event Custom|Server:WaterRune
  (Rune|WaterRune())
  (CallFunction|Server:FireActivity)
  (CallFunction|Server:WaterActivity)
  (Utilities|FlowControl|RetriggerableDelay 1.0)
  (Variables|Spell|SetSpellTable ""))

(event Custom|Server:WaterActivity
  (bind _mywater (Variables|Default|GetMyWater))
  (if (> (Utilities|String|Len (Variables|Spell|GetSpellTable)) 2)
    (Networking|SwitchHasAuthority
      (:Authority
        (Utilities|FlowControl|Sequence
          (:then_1
            (for (_array_element _array_index) _mywater
              (Utilities|IsValid _array_element
                (:Is%20Valid
                  (Variables|Default|SetOverlappingArrayInt _array_index)
                  (if (> (Variables|Default|GetOverlappingArrayInt) -1)
                    (Variables|Default|SetOverlappingArrayInt (- (Variables|Default|GetOverlappingArrayInt) 1))
                    (bind _aswater (Utilities|Casting|CastToWater _array_element))
                    (if (Variables|/Game/NetworkCharacter/Spells/Water/Water.Water_C|GetTransformActive? _aswater)
                      (CallFunction|UnfreezeIcicle _array_element "WBI" :!label _label)
                      (else
                        (Utilities|FlowControl|Sequence
                          (:then_0
                            (Utilities|WaterIcicleMacros _array_element "WBA"))
                          (:then_1
                            (CallFunction|IcicleLaunch _array_element "WBH"))
                          (:then_2
                            (goto _label))
                          (:then_3
                            (CallFunction|MakeFog _array_element "WBBIA" true))
                          (:then_4
                            (CallFunction|MakeFog _array_element "WBBAI" false))
                          (:then_5
                            (CallFunction|MakeShieldorSword _array_element "WIIBI" false)))))))
                (:Is%20Not%20Valid
                  (Utilities|Array|RemoveIndex _mywater _array_index)))))
          (:then_2
            (CallFunction|FreezeAll "WIIW")))))))

(event Custom|Server:FireRune%28Uruz%29
  (Rune|FireRuneActive(Uruz))
  (CallFunction|Server:FireActivity)
  (CallFunction|Server:WaterActivity)
  (Utilities|FlowControl|RetriggerableDelay 1.0)
  (Variables|Spell|SetSpellTable ""))

(event Custom|Server:BallRune%28Teivaz%29
  (Rune|BallRuneActive(Teivaz))
  (CallFunction|Server:FireActivity)
  (CallFunction|Server:WaterActivity)
  (Utilities|FlowControl|RetriggerableDelay 1.0)
  (Variables|Spell|SetSpellTable ""))

(event Custom|Server:FireControll
  (bind _migicoverlap (Utilities|MagicSpawn&Controll 0 "FA" "/Game/WorldMagicElements/Fire.Fire_C")
    (:CaptureMagicAI
      (if (== (Utilities|GetClass _migicoverlap) "/Game/NetworkCharacter/FireBall.FireBall_C")
        (Fire|CaptureFireforAI _migicoverlap)
        (Utilities|FlowControl|Delay 0.05)
        (Variables|Spell|SetSpellTable "")))
    (:CaptureMagicPlayer
      (bind _asfire (Utilities|Casting|CastToFire _migicoverlap))
      (Default|FireListening _asfire self)
      (Variables|Spell|SetSpellTable ""))))

(event Custom|Server:ActiveRune%28Ancuz%29
  (Rune|ActivateRuneActive(Ancuz))
  (CallFunction|Server:FireActivity)
  (CallFunction|Server:WaterActivity)
  (Utilities|FlowControl|RetriggerableDelay 1.0)
  (Variables|Spell|SetSpellTable ""))

(event Custom|Server:StopRune%28Isa%29
  (Rune|StopRuneActive(Isa))
  (Utilities|FlowControl|Sequence
    (:then_0
      (CallFunction|Server:FireActivity)
      (CallFunction|Server:WaterActivity)
      (Utilities|FlowControl|RetriggerableDelay 1.0)
      (Variables|Spell|SetSpellTable ""))))

(event Custom|TakeTarget
  (Utilities|FlowControl|Delay 0.2)
  (Networking|SwitchHasAuthority
    (:Authority
      (bind _outhit (Collision|SphereTraceForObjects (Transformation|GetActorLocation) (+ (Variables|/Game/NetworkCharacter/ClientSideController.ClientSideController_C|GetMouseLocation (Variables|Default|GetClientSideControllerRef)) "0,0.000000,30.000000") 2e+02 (Utilities|Array|MakeArray "ObjectTypeQuery3" "ObjectTypeQuery1") false (Utilities|Array|MakeArray (Variables|/Game/NetworkCharacter/ClientSideController.ClientSideController_C|GetServerSideCharacterRef (Variables|Default|GetClientSideControllerRef))) "None" true "(R=1.000000,G=0.000000,B=0.000000,A=1.000000)" "(R=0.000000,G=1.000000,B=0.000000,A=1.000000)" 0.2))
      (if true
        (if (or (== (Utilities|GetClass (.HitActor (Collision|BreakHitResult _outhit))) "/Game/NetworkCharacter/ServerCharacterController.ServerCharacterController_C") (== (Utilities|GetClass (.HitActor (Collision|BreakHitResult _outhit))) "/Game/AI/BP_AICharecter.BP_AICharecter_C"))
          (bind _output_get (Variables|Default|SetTargetForMissile (.HitActor (Collision|BreakHitResult _outhit))))
          (Development|PrintString (Utilities|GetDisplayName _output_get)))))))

(event Custom|RangeToTarget
  (bind _returnvalue (Transformation|GetActorLocation))
  (Utilities|FlowControl|Delay 0.5)
  (if (not (== (Variables|Default|GetTargetForMissile) 0))
    (bind _returnvalue_2 (Collision|LineTraceForObjects _returnvalue (Transformation|GetActorLocation (Variables|Default|GetTargetForMissile)) (Utilities|Array|MakeArray "ObjectTypeQuery1") false 0 "None" true "(R=1.000000,G=0.000000,B=0.000000,A=1.000000)" "(R=0.000000,G=1.000000,B=0.000000,A=1.000000)" 0.2))
    (if (or (> (Math|Vector|VectorLength (- _returnvalue (Transformation|GetActorLocation (Variables|Default|GetTargetForMissile)))) 1e+03) _returnvalue_2)
      (Utilities|FlowControl|Delay 1.0)
      (Variables|Default|SetTargetForMissile 0)
      (Development|PrintString "target out of range")
      (else
        (Development|PrintString (Utilities|String|BuildString(Float) (Utilities|GetDisplayName (Variables|Default|GetTargetForMissile)) "" (Math|Vector|VectorLength (- _returnvalue (Transformation|GetActorLocation (Variables|Default|GetTargetForMissile))))))))))

(event Custom|Server:WaterControll
  (bind _mywater (Variables|Default|GetMyWater))
  (bind _migicoverlap (Utilities|MagicSpawn&Controll "/Game/NetworkCharacter/Spells/Water/Water.Water_C" "WA" "/Game/NetworkCharacter/Spells/Water/Water.Water_C")
    (:CaptureMagicPlayer
      (if (== (Utilities|GetClass _migicoverlap) "/Game/NetworkCharacter/Spells/Water/Water.Water_C")
        (CallFunction|WaterCapture _migicoverlap)
        (Utilities|FlowControl|Delay 0.01)
        (Variables|Spell|SetSpellTable "")))
    (:RotationControllForPlayer
      (if (== (Utilities|GetClass _migicoverlap) "/Game/NetworkCharacter/Spells/Water/Water.Water_C")
        (if (> (Utilities|Array|LastIndex _mywater) -1)
          (for (_array_element _array_index) _mywater
            (Utilities|IsValid _array_element
              (:Is%20Valid
                (CallFunction|WaterRotation _array_element))
              (:Is%20Not%20Valid
                (Utilities|Array|RemoveIndex _mywater _array_index)))))))))

(event EventTick
  (params (DeltaSeconds :type Float%20%28single-precision%29))
  (Utilities|FlowControl|Sequence
    (:then_0
      (CallFunction|RangetoTarget))
    (:then_1
      (Utilities|FlowControl|Sequence
        (:then_0
          (CallFunction|Server:FireControll))
        (:then_1
          (CallFunction|Server:WaterControll))))
    (:then_2
      (if (Variables|Default|GetThisIsAI)
        _))))

(fn ConstructionScript)

(fn FireRuneActive(Uruz)
  (bind _output_get (Variables|Spell|SetSpellTable (Utilities|String|Append (Variables|Spell|GetSpellTable) "F")))
  (Development|PrintString _output_get))

(fn BallRuneActive(Teivaz)
  (bind _output_get (Variables|Spell|SetSpellTable (Utilities|String|Append (Variables|Spell|GetSpellTable) "B")))
  (Audio|PlaySoundatLocation 0 (Transformation|GetActorLocation) "0, 0, 0" 1.0 1.0 0.0 0 0 0))

(fn ForwardRuneActive(Hagalaz)
  (bind _output_get (Variables|Spell|SetSpellTable (Utilities|String|Append (Variables|Spell|GetSpellTable) "H")))
  (Development|PrintString _output_get))

(fn ActivateRuneActive(Ancuz)
  (bind _output_get (Variables|Spell|SetSpellTable (Utilities|String|Append (Variables|Spell|GetSpellTable) "A")))
  (Development|PrintString _output_get))

(fn CaptureFire
  (params (OverlappingActor :type Actor%20Object%20Reference))
  (bind _output_get (Variables|Default|SetOverlappingActor OverlappingActor))
  (if (Utilities|Enum|Equal(Enum) (Variables|Spell|GetSpellTable) "FA")
    (Utilities|Casting|CastToFireBall _output_get)))

(fn FireBallCompil
  (params (OverlappingActor :type Actor%20Object%20Reference))
  (bind _output_get (Variables|Default|SetOverlappingActor OverlappingActor))
  (bind _asfire_ball (Utilities|Casting|CastToFireBall _output_get))
  (for (_array_element _array_index) (Collision|GetOverlappingActors _asfire_ball "/Game/NetworkCharacter/FireBall.FireBall_C" :!class /Script/Engine.Actor)
    (if (not (>= (* (Variables|/Game/NetworkCharacter/FireBall.FireBall_C|GetFireBatarySettings _asfire_ball) 0.26) 33.0))
      (Actor|DestroyActor _array_element)
      (if (>= _array_index 0)
        (Default|FireBallCompil _asfire_ball)))))

(fn StopRuneActive(Isa)
  (bind _output_get (Variables|Spell|SetSpellTable (Utilities|String|Append (Variables|Spell|GetSpellTable) "I")))
  (Development|PrintString _output_get))

(fn FireBallRotation
  (params (TargetForRot :type Fire%20Ball%20Object%20Reference) (SpawnActorLocation :type Actor%20Object%20Reference))
  (bind _clientsidecontrollerref (Variables|Default|GetClientSideControllerRef))
  (bind _mouselocation (Variables|/Game/NetworkCharacter/ClientSideController.ClientSideController_C|GetMouseLocation _clientsidecontrollerref))
  (bind _output_get (Variables|Default|SetNewVar_0 (Math|Vector|VectorLength (- (Transformation|GetActorLocation SpawnActorLocation) _mouselocation))))
  (Default|FireRotation TargetForRot (+ _mouselocation (Math|Vector|MakeVector 0.0 0.0 (/ _output_get 4.0)))))

(fn OnRepTargetforMissile)

(fn CaptureFireforAI
  (params (OverlappingActor :type Actor%20Object%20Reference))
  (bind _output_get (Variables|Default|SetOverlappingActor OverlappingActor))
  (Utilities|Casting|CastToFireBall _output_get))

(fn FireBallRotationforAI
  (params (OverlappingActor :type Actor%20Object%20Reference))
  (bind _returnvalue (Utilities|Name|MakeLiteralName "Enemy"))
  (bind _firstairef (Variables|Default|GetFirstAIRef))
  (bind _returnvalue_2 (AI|GetBlackboard _firstairef))
  (bind _resultlocation (Class|BlackboardComponent|GetLocationfromEntry _returnvalue_2 _returnvalue))
  (Utilities|FlowControl|Sequence
    (:then_0
      (if (Variables|Default|GetFlameON)
        (Variables|Default|SetAITargetVelocity "0, 0, 0")
        (else
          (bind _asserver_character_controller (Utilities|Casting|CastToServerCharacterController (AI|Components|Blackboard|GetValueasObject (AI|GetBlackboard (Variables|Default|GetFirstAIRef)) (Utilities|Name|MakeLiteralName "Enemy"))))
          (Variables|Default|SetAITargetVelocity (Transformation|GetVelocity _asserver_character_controller)))))
    (:then_1
      (bind _output_get (Variables|Default|SetOverlappingActor OverlappingActor))
      (bind _asfire_ball (Utilities|Casting|CastToFireBall _output_get))
      (bind _output_get_2 (Variables|Default|SetNewVar_0 (Math|Vector|VectorLength (- (Transformation|GetActorLocation) _resultlocation))))
      (Default|FireRotation _asfire_ball (+ (Variables|Default|GetAITargetVelocity) (+ _resultlocation (Math|Vector|MakeVector 0.0 0.0 (/ _output_get_2 1e+01))))))))

(fn WaterCapture
  (params (OverlappingActor :type Actor%20Object%20Reference))
  (bind _output_get (Variables|Default|SetOverlappingActor OverlappingActor))
  (bind _aswater (Utilities|Casting|CastToWater _output_get))
  (Utilities|Array|Add (Variables|Default|GetMyWater) _aswater)
  (Default|HomingMissile _aswater (Variables|/Game/NetworkCharacter/ClientSideController.ClientSideController_C|GetServerSideCharacterRef (Variables|Default|GetClientSideControllerRef)) self))

(fn WaterCaptureforAI)

(fn WaterRotation
  (params (OverlappingActor :type Actor%20Object%20Reference))
  (bind _output_get (Variables|Default|SetOverlappingActor OverlappingActor))
  (bind _aswater (Utilities|Casting|CastToWater _output_get))
  (Default|WaterRotation _aswater (Variables|/Game/NetworkCharacter/ClientSideController.ClientSideController_C|GetMouseLocation (Variables|Default|GetClientSideControllerRef))))

(fn WaterRune()
  (bind _output_get (Variables|Spell|SetSpellTable (Utilities|String|Append (Variables|Spell|GetSpellTable) "W")))
  (Development|PrintString _output_get))

(fn IcicleLaunch
  (params (OverlappingActor :type Actor%20Object%20Reference) (IcicleLaunchWord :type String))
  (bind _output_get (Variables|Default|SetOverlappingActor OverlappingActor))
  (if (Utilities|Enum|Equal(Enum) (Variables|Spell|GetSpellTable) IcicleLaunchWord)
    (bind _aswater (Utilities|Casting|CastToWater _output_get))
    (Default|HomingMissileOff _aswater)))

(fn UnfreezeIcicle
  (params (OverlappingActor :type Actor%20Object%20Reference) (UnfreezeWord :type String))
  (bind _output_get (Variables|Default|SetOverlappingActor OverlappingActor))
  (if (Utilities|Enum|Equal(Enum) (Variables|Spell|GetSpellTable) UnfreezeWord)
    (bind _aswater (Utilities|Casting|CastToWater _output_get))
    (Default|Unfreeze _aswater (Variables|/Game/NetworkCharacter/ClientSideController.ClientSideController_C|GetServerSideCharacterRef (Variables|Default|GetClientSideControllerRef)))))

(fn FreezeAll
  (params (SpellWord :type String))
  (if (Utilities|String|Contains (Variables|Spell|GetSpellTable) SpellWord false true)
    (for _array_element (Variables|Default|GetActorsOverlap)
      (bind _astest_char (Utilities|Casting|CastToTestChar _array_element))
      (if (Variables|/Game/AdvancedLocomotionV3/Blueprints/TestChar.TestChar_C|GetIsWet _astest_char)
        (Default|FreezeCharacter _astest_char)))))

(fn MakeFog
  (params (OverlappingActor :type Actor%20Object%20Reference) (SpellWord :type String) (FogOn? :type Boolean))
  (bind _output_get (Variables|Default|SetOverlappingActor OverlappingActor))
  (if (Utilities|Enum|Equal(Enum) (Variables|Spell|GetSpellTable) SpellWord)
    (bind _aswater (Utilities|Casting|CastToWater _output_get))
    (if (Math|Boolean|NotEqual(Boolean) FogOn? (Components|Activation|IsActive (Variables|/Game/NetworkCharacter/Spells/Water/Water.Water_C|GetFog _aswater)))
      (Default|FogActivate? _aswater FogOn?)
      (Variables|Spell|SetSpellTable ""))))

(fn MakeShieldorSword
  (params (OverlappingActor :type Actor%20Object%20Reference) (SpellWord :type String) (IfTrueShildOff&SwordOn :type Boolean))
  (bind _self self)
  (bind _clientsidecontrollerref (Variables|Default|GetClientSideControllerRef))
  (bind _serversidecharacterref (Variables|/Game/NetworkCharacter/ClientSideController.ClientSideController_C|GetServerSideCharacterRef _clientsidecontrollerref))
  (bind _output_get (Variables|Default|SetOverlappingActor OverlappingActor))
  (if (Utilities|Enum|Equal(Enum) (Variables|Spell|GetSpellTable) SpellWord)
    (bind _aswater (Utilities|Casting|CastToWater _output_get))
    (if IfTrueShildOff&SwordOn
      (Default|IceSword _aswater _serversidecharacterref _self)
      (else
        (Default|IceShield _aswater _serversidecharacterref _self)))))